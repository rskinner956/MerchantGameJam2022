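; BaseEnemy is a base enemy character Blueprint that provides helper functions for movement speed and target-point cycling.
; UpdateWalkSpeed sets the CharacterMovement max walk speed.
; GetNextTargetPoint returns the array entry at the current index, then increments it, resetting only when it equals the array length, so one read per cycle is out of range.
; Its event graph and construction script hold no logic.
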(fn `GetNextTargetPoint`
  (returns (TargetPoint :type "Vector Structure"))
  (locals (nextLocation :type "Vector Structure"))
  (bind _targetpoints_arr (`self.TargetPoints_Arr`))
  (bind _currindex (`self.CurrIndex`))
  (set `local.nextLocation` (`|GetArrayItem` _targetpoints_arr _currindex))
  (if (== _currindex (`KismetArrayLibrary.Array_Length` _targetpoints_arr))
    (set `self.CurrIndex` 0)
    (else
      (`/Engine/EditorBlueprintResources/StandardMacros.IncrementInt` (`self.CurrIndex`)
        (:`  `
          _))))
  (return (`local.nextLocation`)))

(fn `UpdateWalkSpeed`
  (params (NewWalkSpeed :type "Float (double-precision)"))
  (set `CharacterMovementComponent.MaxWalkSpeed` NewWalkSpeed (`self.CharacterMovement`)))

(fn `UserConstructionScript`)